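; Game mode for the multiplayer main menu that tracks lobby player controllers and shares the player name list.
; On post-login it stores the controller, unique net ID and name, copies the ID and name onto the controller, then calls UpdatePlayerList on every connected controller.
; Logout only removes the controller, leaving the ID and name lists unchanged and sending no list update.
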(event EventBeginPlay)

(event EventTick
  (params (DeltaSeconds :type Float%20%28single-precision%29)))

(event EventPostLogin
  (params (NewPlayer :type Player%20Controller%20Object%20Reference))
  (bind _playername (Class|AdvancedSessionsLibrary|GetPlayerName NewPlayer))
  (bind _uniquenetid (Class|AdvancedSessionsLibrary|GetUniqueNetID NewPlayer))
  (bind _returnvalue (Class|AdvancedSessionsLibrary|ToUniqueNetIDRepl(BPUniqueID) _uniquenetid))
  (bind _asbp_player_controller_lobby (Utilities|Casting|CastToBP_PlayerController_Lobby NewPlayer))
  (Utilities|Array|Add (Variables|Default|GetConnectedPlayers) _asbp_player_controller_lobby)
  (Variables|/Game/Blueprints/BP_PlayerController_Lobby.BP_PlayerController_Lobby_C|SetUniqNetID _asbp_player_controller_lobby _returnvalue)
  (Variables|/Game/Blueprints/BP_PlayerController_Lobby.BP_PlayerController_Lobby_C|SetPlayerName _asbp_player_controller_lobby _playername)
  (Utilities|Array|Add (Variables|Default|GetConnectedPlayerIDs) _returnvalue)
  (Utilities|Array|Add (Variables|Default|GetConnectedPlayerNames) _playername)
  (for _array_element (Variables|Default|GetConnectedPlayers)
    (Default|UpdatePlayerList _array_element (Variables|Default|GetConnectedPlayerNames))))

(event EventOnLogout
  (params (ExitingController :type Controller%20Object%20Reference))
  (bind _asbp_player_controller_lobby (Utilities|Casting|CastToBP_PlayerController_Lobby ExitingController))
  (Utilities|Array|RemoveItem (Variables|Default|GetConnectedPlayers) _asbp_player_controller_lobby))

(fn ConstructionScript)